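; BP_Projectile is a projectile that destroys enemies and scores points for its shooter.
; Each Tick it sweeps along world X at a multiple of the player pawn's current Speed, without delta-time scaling.
; Overlapping a BP_Enemy destroys both actors and adds a fixed amount to the Shooter's Score.
; A BulletDrop function computes a forward offset with speed-squared downward drop, but nothing in this file calls it.
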(event OnComponentBeginOverlap(projectile)
  (params (OverlappedComponent :type Primitive%20Component%20Object%20Reference) (OtherActor :type Actor%20Object%20Reference) (OtherComp :type Primitive%20Component%20Object%20Reference) (OtherBodyIndex :type Integer) (bFromSweep :type Boolean) (SweepResult :type Hit%20Result%20Structure%20%28by%20ref%29))
  (bind _shooter (Variables|Default|Getshooter))
  (bind _asbp_enemy (Utilities|Casting|CastToBP_Enemy OtherActor))
  (Actor|DestroyActor _asbp_enemy)
  (Actor|DestroyActor)
  (Variables|/Game/InfiniteMatrix/Blueprints/BP_Player.BP_Player_C|SetScore _shooter (+ (Variables|/Game/InfiniteMatrix/Blueprints/BP_Player.BP_Player_C|GetScore _shooter) 2e+01)))

(event EventBeginPlay)

(event Collision|EventActorBeginOverlap
  (params (OtherActor :type Actor%20Object%20Reference)))

(event EventTick
  (params (DeltaSeconds :type Float%20%28single-precision%29))
  (bind _asbp_player (Utilities|Casting|CastToBP_Player (Game|Player|GetPlayerPawn 0)))
  (Transformation|AddActorWorldOffset (Math|Vector|MakeVector (* (Variables|/Game/InfiniteMatrix/Blueprints/BP_Player.BP_Player_C|Getspeed _asbp_player) 3.0) 0.0 0.0) true))

(fn ConstructionScript)

(fn BulletDrop
  (params (speed :type Float%20%28double-precision%29))
  (bind _returnvalue (* speed 3.0))
  (return _returnvalue (/ (* _returnvalue _returnvalue -0.01) 3.0)))